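; BP_MuffinCamera is a follow camera that tracks the player's BP_Muffin pawn along the vertical axis.
; On BeginPlay it sets the first player controller's view target to GameCamera.
; Every Tick, MoveCamera casts the player pawn to BP_Muffin and copies its Z position onto this actor, keeping X and Y unchanged.
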(event EventBeginPlay
  ;[1 1 1] 将相机的镜头对准玩家
  (Game|Player|SetViewTargetwithBlend (Game|GetPlayerController 0) (Variables|Default|GetGameCamera) 0.0 "VTBlend_Linear" 0.0 false))

(event EventTick
  (params (DeltaSeconds :type Float%20%28single-precision%29))
  ;[1 1 1] 镜头实时跟随玩家
  (CallFunction|MoveCamera))

(fn ConstructionScript)

(fn MoveCamera
  (bind _returnvalue (Transformation|GetActorLocation))
  ;[1 1 1] 将相机的Z轴设置为玩家的Z轴，其他保持不变，以实现镜头跟随玩家移动
  (bind _asbp_muffin (Utilities|Casting|CastToBP_Muffin (Game|Player|GetPlayerPawn 0)))
  (Transformation|SetActorLocation (Math|Vector|MakeVector (.x _returnvalue) (.y _returnvalue) (.z (Transformation|GetActorLocation _asbp_muffin))) false false))