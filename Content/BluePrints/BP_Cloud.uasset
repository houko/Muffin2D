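; BP_Cloud is a cloud actor that shows a randomly chosen cloud shape on its CloudPlane mesh.
; The construction script takes the plane's first material, creates a dynamic instance from it, sets that instance's Texture parameter to a random entry from CloudShapes, then applies it to the plane.
; All work happens at construction, and BeginPlay is empty.
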(event EventBeginPlay)

(fn ConstructionScript
  (Utilities|FlowControl|Sequence
    (:then_0
      (CallFunction|SetMatInterface))
    (:then_1
      (CallFunction|SetMatInstance))
    (:then_2
      (CallFunction|CreateRandomCloud))))

(fn SetMatInterface
  (Variables|Default|SetMatInterface (Utilities|Array|Get(acopy) (Rendering|Material|GetMaterials (Variables|Default|GetCloudPlane)))))

(fn CreateRandomCloud
  (bind _cloudshapes (Variables|Default|GetCloudShapes))
  (Utilities|FlowControl|Sequence
    (:then_0
      ;[1 1 1] 随机贴图
      (Rendering|Material|SetTextureParameterValue (Variables|Default|GetMatInstance) "Texture" (Utilities|Array|Get(acopy) _cloudshapes (Math|Random|RandomInteger (Utilities|Array|Length _cloudshapes)))))
    (:then_1
      ;[1 1 1] 设置贴图
      (Rendering|Material|SetMaterial (Variables|Default|GetCloudPlane) 0 (Variables|Default|GetMatInstance)))))

(fn SetMatInstance
  (bind _returnvalue (Rendering|Material|CreateDynamicMaterialInstance (Variables|Default|GetMatInterface) "None" :!class /Script/Engine.KismetMaterialLibrary))
  (Variables|Default|SetMatInstance _returnvalue))