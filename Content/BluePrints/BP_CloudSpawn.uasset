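; BP_CloudSpawn is a rising spawner that creates BP_Cloud actors as BP_Character reaches it.
; When a BP_Character overlaps it, SpawnCloud places a cloud with random Y within SpawnArea's bounds, keeping the area's X and Z.
; After each spawn the spawner moves itself up by SpawnSpacing, stacking clouds vertically.
; SpawnInStartGame repeats this for an initial batch but is not called within this Blueprint.
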(event Collision|EventActorBeginOverlap
  (params (OtherActor :type Actor%20Object%20Reference))
  (bind _asbp_character (Utilities|Casting|CastToBP_Character OtherActor))
  (Utilities|IsValid _asbp_character
    (:Is%20Valid
      (CallFunction|SpawnCloud))))

(fn ConstructionScript)

(fn SpawnCloud
  (bind _spawnarea (Variables|Default|GetSpawnArea))
  (bind (_origin _boxextent) (Collision|GetComponentBounds _spawnarea))
  (bind _returnvalue (Transformation|GetWorldLocation _spawnarea))
  ;[1 1 1] 随机生成点
  (bind _output_get (Variables|Default|SetSpawnLocation (Math|Vector|MakeVector (.x _returnvalue) (.y (Math|Random|RandomPointinBoundingBox _origin _boxextent)) (.z _returnvalue))))
  (Game|SpawnActorfromClass "/Game/BluePrints/BP_Cloud.BP_Cloud_C" (Math|Conversions|ToTransform(Vector) _output_get) "Undefined" 0 0) ; 生成云彩
  (Transformation|AddActorWorldOffset (Math|Vector|MakeVector 0.0 0.0 (Variables|Default|GetSpawnSpacing))) ; 将生成器上升
)

(fn SpawninStartGame
  (for _index (range 0 (Variables|Default|GetInitialSpawnCount))
    (CallFunction|SpawnCloud)))