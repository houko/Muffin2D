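; Player character for a cloud-jumping game that follows the mouse cursor along the Y axis and scores a point per launch.
; Each tick sets walk speed for air or ground, checks for death and adds clamped movement input from the deprojected cursor position.
; Once started, not falling means death, which clears the score and disables input.
; Reset clears the game state and resets the first BP_CloudSpawn found.
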(event EventBeginPlay
  ;[1 1 1] 开始游戏时给Player赋值并显示鼠标
  (CallFunction|ShowCursor))

(event EventTick
  (params (DeltaSeconds :type Float%20%28single-precision%29))
  ;[1 1 1] Tick时玩家跟随鼠标移动
  (CallFunction|SetCharacterSpeed)
  (CallFunction|CheckDead)
  (CallFunction|MoveTowardsCursor))

(fn ConstructionScript)

(fn ShowCursor
  (Variables|/Script/Engine.PlayerController|SetbShowMouseCursor (Game|GetPlayerController 0) true))

(fn MoveTowardsCursor
  ;[1 1 1] 使玩家跟随鼠标移动
  (bind _movedirection (CallFunction|GetMoveDirection))
  (LocalVariables|SetMoveDirection (Math|Vector|MakeVector 0.0 _movedirection 0.0))
  (Pawn|Input|AddMovementInput (LocalVariables|GetMoveDirection) 1.0 false))

(fn GetMoveDirection
  (bind _returnvalue (Game|GetPlayerController 0))
  (return (Math|Float|Clamp(Float) (- (.y (.WorldLocation (Game|Player|ConvertMouseLocationToWorldSpace _returnvalue))) (.y (Transformation|GetActorLocation _returnvalue))) -1.0)))

(fn LaunchGameonClick
  (CallFunction|Launch))

(fn SetCharacterSpeed
  (bind _charactermovement (Variables|Character|GetCharacterMovement))
  ;[1 1 1] 根据玩家的状态设置它的速度（每帧调用，需要设置CharacterMovement参数）
  (if (AI|Components|NavMovement|IsFalling (Variables|Character|GetCharacterMovement))
    (Variables|/Script/Engine.CharacterMovementComponent|SetMaxWalkSpeed _charactermovement (Variables|Default|GetAirSpeed))
    (else
      (Variables|/Script/Engine.CharacterMovementComponent|SetMaxWalkSpeed _charactermovement (Variables|Default|GetGroundSpeed)))))

(fn Launch
  (Character|LaunchCharacter (Variables|Default|GetLaunchVelocity) false true)
  (CallFunction|AddScore))

(fn AddScore
  ;[1 1 1] 增加分数
  (Math|Integer|IncrementInt (Variables|Default|GetScore)))

(fn GetScore
  (return (Variables|Default|GetScore)))

(fn GameOver
  (Variables|BP_Character_C|SetScore self 0)
  (Input|DisableInput 0))

(fn CheckDead
  ;[1 1 1] 如果游戏开始了，但玩家没有在下落状态则游戏结束
  (if (Variables|Default|GetIsStart)
    (if (not (AI|Components|NavMovement|IsFalling (Variables|Character|GetCharacterMovement self)))
      (Variables|Default|SetIsDead true)
      (CallFunction|GameOver))))

(fn Reset
  ;[1 1 1] 重置游戏状态
  (Utilities|FlowControl|Sequence
    (:then_0
      (Variables|Default|SetIsStart false))
    (:then_1
      (Variables|Default|SetIsDead false))
    (:then_2
      (Variables|Default|SetScore 0))
    (:then_3
      (bind _outactors (Actor|GetAllActorsOfClass "/Game/BluePrints/BP_CloudSpawn.BP_CloudSpawn_C"))
      (Default|Reset (Utilities|Array|Get(acopy) _outactors)))))